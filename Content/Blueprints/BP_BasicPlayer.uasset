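; BP_BasicPlayer is a basic player character with walking, jumping and mouse look driven by input mappings.
; Forward/Backward and Right/Left axes add movement input along the actor's forward and right vectors, and the Jump action triggers a jump on press.
; Look axes feed controller yaw and pitch input directly, with no scaling, and the construction script is empty.
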(event Input|ActionEvents|InputActionJump
  (params (Key :type Key%20Structure :default "None"))
  ;[0.7119 1 0.805] Movement Jump
  (:Pressed
    (Character|Jump)))

(event Input|AxisEvents|InputAxisForward/Backward
  (params (AxisValue :type Float%20%28single-precision%29))
  ;[0.7427 0.7503 1] Movement Forward/Back/Right/Left
  (Pawn|Input|AddMovementInput (Transformation|GetActorForwardVector) AxisValue false))

(event Input|AxisEvents|InputAxisRight/Left
  (params (AxisValue :type Float%20%28single-precision%29))
  ;[0.7427 0.7503 1] Movement Forward/Back/Right/Left
  (Pawn|Input|AddMovementInput (Transformation|GetActorRightVector) AxisValue false))

(event Input|AxisEvents|InputAxisLook_Left/Right
  (params (AxisValue :type Float%20%28single-precision%29))
  ;[1 1 1] MouseLook Right/Left
  (Pawn|Input|AddControllerYawInput AxisValue))

(event Input|AxisEvents|InputAxisLook_Up/Down
  (params (AxisValue :type Float%20%28single-precision%29))
  ;[1 1 1] MouseLook Up/Down
  (Pawn|Input|AddControllerPitchInput AxisValue))

(fn ConstructionScript)